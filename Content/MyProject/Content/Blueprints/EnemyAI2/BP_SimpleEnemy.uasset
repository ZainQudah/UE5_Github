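; BP_SimpleEnemy is a simple enemy pawn that wanders and chases the player.
; From BeginPlay it moves to random navigable points around itself, pausing after each successful arrival before picking the next.
; A PawnSensing sighting of any pawn sets IsSeeingPlayer and starts an AIMoveTo toward the player character.
; If that chase move fails, it clears the flag and resumes wandering after a retriggerable delay.
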(event OnSeePawn(PawnSensing)
  (params (Pawn :type Pawn%20Object%20Reference))
  ;[1 1 1] FollowPlayer on Sight
  (Variables|Default|SetisSeeingPlayer true)
  (CallFunction|FollowPlayer))

(event Custom|FollowPlayer
  ;[1 1 1] FollowPlayer on Sight
  (if (Variables|Default|GetisSeeingPlayer)
    (AI|AIMoveTo self "0, 0, 0" (Game|GetPlayerCharacter 0) 7e+01 false
      (:OnFail
        (Variables|Default|SetisSeeingPlayer false)
        (Utilities|FlowControl|RetriggerableDelay 3.0)
        (CallFunction|MovetoRandomLocation)))))

(event Custom|MoveToRandomLocation
  (bind _randomlocation (Class|NavigationSystemV1|GetRandomLocationinNavigableRadius (Transformation|GetActorLocation) 1e+03 0 0))
  (AI|AIMoveTo self _randomlocation 0 5.0 false
    (:OnSuccess
      (Utilities|FlowControl|Delay 3.0)
      (CallFunction|MovetoRandomLocation))))

(event Collision|EventActorBeginOverlap
  (params (OtherActor :type Actor%20Object%20Reference)))

(event EventBeginPlay
  (CallFunction|MovetoRandomLocation))

(event EventTick
  (params (DeltaSeconds :type Float%20%28single-precision%29)))

(fn ConstructionScript)