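; Practice cube actor that moves between two points, changes color, and pushes the third-person player away on contact.
; A dynamic material turns the target color on the 1 key and black when the player overlaps or hits it.
; Contact also applies an impulse along the Hit event's normal, negated.
; A Timeline lerps the location, while a looping timer flips a direction flag read only by disconnected movement code.
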(event Custom|ChangeDirection
  ;[1 1 1] Custom Event To Switch Time - 5
  (Utilities|FlowControl|FlipFlop
    (:A
      (Variables|Default|SetisMovingForward false))
    (:B
      (Variables|Default|SetisMovingForward true))))

(event EventBeginPlay
  (Utilities|FlowControl|Sequence
    (:then_0
      ;[1 1 1] Change Color on Button Press - 1
      (bind _returnvalue (Rendering|Material|CreateDynamicMaterialInstance "/Game/Blueprints/EnemyAI2/DynamicMAterial.DynamicMAterial" "None" "None" :!class /Script/Engine.KismetMaterialLibrary))
      (Variables|Default|SetCubeMaterial _returnvalue)
      (Rendering|Material|SetMaterial (Variables|Debug|GetStaticMeshComponent) 0 (Variables|Default|GetCubeMaterial))
      ;[1 1 1] Custom Event To Switch Time - 5
      (Utilities|Time|SetTimerbyEvent (delegate Custom|ChangeDirection) 2.0 true))
    (:then_1
      ;[1 1 1] Move Between 2 Points - 7]
      (bind _alpha (Timeline|Timeline PlayFromStart)
        (:Update
          (Transformation|SetActorLocation (Math|Vector|Lerp(Vector) (Variables|Default|GetPointA) (Variables|Default|GetPointB) _alpha) false false))))))

(event Collision|EventActorBeginOverlap
  (params (OtherActor :type Actor%20Object%20Reference))
  ;[1 1 1] Change Cube Color on Overlap/Collision - 2
  (bind _asbp_third_person_character (Utilities|Casting|CastToBP_ThirdPersonCharacter (stale Collision|EventHit Other)))
  (Rendering|Material|SetVectorParameterValue :self (Variables|Default|GetCubeMaterial) :ParameterName "Color" :!class /Script/Engine.MaterialInstanceDynamic)
  ;[1 1 1] Push Player Away - 6
  (Physics|AddImpulse (Variables|/Script/Engine.Character|GetCharacterMovement _asbp_third_person_character) (* (stale Collision|EventHit HitNormal) -1e+03) true))

(event Collision|EventHit
  (params (MyComp :type Primitive%20Component%20Object%20Reference) (Other :type Actor%20Object%20Reference) (OtherComp :type Primitive%20Component%20Object%20Reference) (bSelfMoved :type Boolean) (HitLocation :type Vector :default "0, 0, 0") (HitNormal :type Vector :default "0, 0, 0") (NormalImpulse :type Vector :default "0, 0, 0") (Hit :type Hit%20Result%20Structure%20%28by%20ref%29))
  ;[1 1 1] Change Cube Color on Overlap/Collision - 2
  (bind _asbp_third_person_character (Utilities|Casting|CastToBP_ThirdPersonCharacter Other))
  (Rendering|Material|SetVectorParameterValue :self (Variables|Default|GetCubeMaterial) :ParameterName "Color" :!class /Script/Engine.MaterialInstanceDynamic)
  ;[1 1 1] Push Player Away - 6
  (Physics|AddImpulse (Variables|/Script/Engine.Character|GetCharacterMovement _asbp_third_person_character) (* HitNormal -1e+03) true))

(event EventTick
  (params (DeltaSeconds :type Float%20%28single-precision%29)))

(event Input|KeyboardEvents|1
  (params (Key :type Key%20Structure :default "None"))
  ;[1 1 1] Change Color on Button Press - 1
  (:Pressed
    (Rendering|Material|SetVectorParameterValue (stale EventBeginPlay _returnvalue) "Color" (Variables|Default|GetTargetColor) :!class /Script/Engine.MaterialInstanceDynamic)
    (Rendering|Material|SetMaterial (Variables|Debug|GetStaticMeshComponent) 0 (Variables|Default|GetCubeMaterial))
    ;[1 1 1] Custom Event To Switch Time - 5
    (Utilities|Time|SetTimerbyEvent (delegate Custom|ChangeDirection) 2.0 true)))

(fn ConstructionScript)